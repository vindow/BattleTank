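; Mortar actor built from turret and barrel parts, with a tank aiming component and a health bar widget.
; On BeginPlay it initializes TankAiming with its Turret and Barrel, then casts the widget component's user widget to HealthBar_BP.
; It passes itself to that health bar as the Tank reference, reusing the tank UI for the mortar.
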(event `self.ReceiveBeginPlay`
  (`TankAimingComponent.Initialize` (`self.TankAiming`) (`self.Turret`) (`self.Barrel`))
  (`self.InitializeHealthBar`))

(fn `InitializeHealthBar`
  (bind _ashealth_bar_bp (cast `/Game/Blueprints/HealthBar_BP` (`WidgetComponent.GetUserWidgetObject` (`self.Widget`))))
  (set `/Game/Blueprints/HealthBar_BP.Tank` self _ashealth_bar_bp))

(fn `UserConstructionScript`)